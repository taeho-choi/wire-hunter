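; Player character Blueprint with the aiming stage of a wire hook, fired by right mouse.
; BeginPlay hides and resets the Wire cable; right-click traces from the camera for world objects with persistent debug drawing.
; The character turns toward the hit location without checking for a hit.
; With controller yaw enabled it also pitches, waits, then levels via timeline while setting Hooked and WireLocation; otherwise it yaws and sets them immediately.
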(event `self.ReceiveTick`
  (params (DeltaSeconds :type "Float (single-precision)")))

(event `self.ReceiveBeginPlay`
  (bind _wire (`self.Wire`))
  ;[1 1 1] Set Cable Parameters
  (`SceneComponent.SetVisibility` _wire false false)
  (set `CableComponent.CableLength` 0.0 _wire)
  (set `CableComponent.CableWidth` 2.0 _wire)
  (set `CableComponent.EndLocation` (120.0 10.0 60.0) _wire))

(event `Key|RightMouseButton`
  (params (Key :type "Key Structure"))
  (bind (_returnvalue_roll _returnvalue_pitch _returnvalue_yaw) (`KismetMathLibrary.BreakRotator` (`self.K2_GetActorRotation`)))
  (bind _camera (`self.Camera`))
  (bind _returnvalue (`SceneComponent.K2_GetComponentLocation` _camera))
  (:`Pressed`
    (bind _outhit (`KismetSystemLibrary.LineTraceSingleForObjects` :`Start` _returnvalue :`End` (+ _returnvalue (* (`SceneComponent.GetForwardVector` _camera) 3500.0)) :`ObjectTypes` (`|MakeArray` "ObjectTypeQuery1" "ObjectTypeQuery2" :!type "EObjectTypeQuery Enum") :`DrawDebugType` "Persistent"))
    (if true
      (if (`self.bUseControllerRotationYaw`)
        (bind (_bblockinghit _binitialoverlap _time _distance _location) (`GameplayStatics.BreakHitResult` _outhit))
        (bind (_returnvalue_roll_2 _returnvalue_pitch_2 _returnvalue_yaw_2) (`KismetMathLibrary.BreakRotator` (`KismetMathLibrary.FindLookAtRotation` (`self.K2_GetActorLocation`) _location)))
        (`self.K2_SetActorRotation` (`KismetMathLibrary.MakeRotator` 0.0 _returnvalue_pitch_2 _returnvalue_yaw_2))
        (`KismetSystemLibrary.Delay` 7.0)
        (bind (_direction _time_2) (`Timeline|타임라인_0` :!via `PlayFromStart`)
          (:`Update`
            (`self.K2_SetActorRotation` (`KismetMathLibrary.RLerp` (`self.K2_GetActorRotation`) (`KismetMathLibrary.MakeRotator` _returnvalue_roll 0.0 _returnvalue_yaw) _time_2))))
        (else
          (bind (_returnvalue_roll_3 _returnvalue_pitch_3 _returnvalue_yaw_3) (`KismetMathLibrary.BreakRotator` (`KismetMathLibrary.FindLookAtRotation` (`self.K2_GetActorLocation`) _location)))
          (`self.K2_SetActorRotation` (`KismetMathLibrary.MakeRotator` 0.0 0.0 _returnvalue_yaw_3))))
      (set `self.Hooked` true)
      (set `self.WireLocation` _location))))

(fn `UserConstructionScript`)